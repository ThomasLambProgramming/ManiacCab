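; Customer pickup spot for a taxi game that hands a ride to the player's BP_Cabbie when it stops inside.
; On BeginPlay it gets a destination from BP_RideManager, derives a timer from distance via a curve, and calculates the fare.
; Distance-based ride type sets the fare rate and colours the ring and coin through dynamic materials.
; Tick polls for pickup, reveals the drop-off and destroys itself, also self-destructing whenever the cab already carries a customer.
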(event `self.ReceiveBeginPlay`
  (bind (_customerdata_time _customerdata_fare _customerdata_destination) (break `/Game/I01_Core/Data/S_CustomerData` (`self.CustomerData`)))
  (bind _returnvalue (`GameplayStatics.GetActorOfClass` "/Game/I01_Core/Blueprints/GameLogic/BP_RideManager.BP_RideManager_C"))
  (bind _output_get (set `self.RideManager` _returnvalue))
  (set `self.As BP Cabbie` (`/Game/I01_Core/Blueprints/GameLogic/BP_RideManager.BP_Cabbie` _output_get))
  (`self.CreateCustomerData`)
  (set `self.DropOffPoint` (`/Game/I01_Core/Blueprints/GameLogic/BP_RideManager.FindDropOffSpot` (`self.RideManager`) _customerdata_destination)))

(event `self.ReceiveTick`
  (params (DeltaSeconds :type "Float (single-precision)"))
  (bind _as_bp_cabbie (`self.As BP Cabbie`))
  (bind _as_bp_cabbie_2 (`self.As BP Cabbie`))
  (`self.RideManager`
    (:`then`
      (if (and (`KismetSystemLibrary.IsValid` _as_bp_cabbie) (not (`/Game/I01_Core/Blueprints/Car/BP_Cabbie.HoldingCustomer` _as_bp_cabbie)))
        (if (and (`self.IsOverlappingActor` _as_bp_cabbie_2) (not (`/Game/I01_Core/Blueprints/Car/BP_Cabbie.IsCarMoving` _as_bp_cabbie_2)))
          ;[1 0.2604 0.2604] Will be replaces with picking up anim and UI anim calls
          (`/Engine/EditorBlueprintResources/StandardMacros.DoOnce` false
            (:`Completed`
              (set `self.HasStopped` true)
              (`self.SetActorHiddenInGame` (`self.DropOffPoint`) false)
              (`/Game/I01_Core/Blueprints/Car/BP_Cabbie.SetupRide` (`self.As BP Cabbie`) (`self.CustomerData`))
              (set `self.HasStopped` false)
              (`self.K2_DestroyActor` self))))
        (else
          (`self.K2_DestroyActor` self))))
    (:`else`)))

(fn `CreateCustomerData`
  (locals (Location :type "/Game/I01_Core/Data/E_Locations Enum") (Distance :type Integer) (RideTimer :type Integer))
  (bind _distance (`local.Distance`))
  (bind _location (`/Game/I01_Core/Blueprints/GameLogic/BP_RideManager.AssignLocation` (`self.RideManager`)))
  (set `local.Location` _location)
  (set `local.Distance` (`KismetMathLibrary.Round` (`self.GetDistanceTo` (`/Game/I01_Core/Blueprints/GameLogic/BP_RideManager.FindDropOffSpot` (`self.RideManager`) (`local.Location`)))))
  (set `local.RideTimer` (`KismetMathLibrary.Round` (`CurveFloat.GetFloatValue` (`self.CurveTable`) (/ (`KismetMathLibrary.Conv_IntToDouble` (`local.Distance`)) 10000.0))))
  (`self.UpdateMaterials` _distance)
  (set `self.CustomerData` (make `/Game/I01_Core/Data/S_CustomerData` (`local.RideTimer`) (`self.EvaluateFare` _distance (`local.RideTimer`)) (`local.Location`))))

(fn `EvaluateFare`
  (params (Distance :type Integer) (Time :type Integer))
  (returns (Fare :type "Float (double-precision)"))
  (return (* (`KismetMathLibrary.Round` (* (* (/ (/ Distance 100) Time) (select `int` (`/Game/I01_Core/Blueprints/GameLogic/BP_RideManager.EvaluateRideType` (`self.RideManager`) (`local.Distance`)) :`0` 10.0 :`1` 18.0 :`2` 22.0 :`3` 27.0)) 100.0)) 0.01)) ; 92.24
)

(fn `UpdateMaterials`
  (params (Distance :type Integer))
  (bind _output_get (set `self.MaterialColour` (select `int` (`/Game/I01_Core/Blueprints/GameLogic/BP_RideManager.EvaluateRideType` (`self.RideManager`) Distance) :`0` (struct :`R` 0.434154 :`G` 0.004391 :`B` 0.016807 :`A` 1.0) :`1` (struct :`R` 0.756863 :`G` 0.137255 :`B` 0.039216 :`A` 1.0) :`2` (struct :`R` 0.756863 :`G` 0.604145 :`B` 0.082102 :`A` 1.0) :`3` (struct :`R` 0.07296 :`G` 0.541667 :`B` 0.026602 :`A` 1.0) :!type "LinearColor Structure")))
  (`MaterialInstanceDynamic.SetVectorParameterValue` (`self.RingMaterial`) "Colour" _output_get)
  (`MaterialInstanceDynamic.SetVectorParameterValue` (`self.CoinMaterial`) "Colour" _output_get))

(fn `UserConstructionScript`
  (bind _returnvalue (`PrimitiveComponent.CreateDynamicMaterialInstance` (`self.StaticMesh`) 0 "/Game/I01_Core/Assets/Materials/MI_CustomerPickup.MI_CustomerPickup" "None"))
  (bind _output_get (set `self.RingMaterial` _returnvalue))
  (`MaterialInstanceDynamic.SetVectorParameterValue` _output_get "Colour" (`self.MaterialColour`))
  (bind _returnvalue_2 (`PrimitiveComponent.CreateDynamicMaterialInstance` (`self.Coin`) 0 "/Game/I01_Core/Assets/Materials/MI_PickupSpot.MI_PickupSpot" "None"))
  (set `self.CoinMaterial` _returnvalue_2))