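; BP_DropOff is a customer drop-off marker for cab rides, hidden at start and labelled with its Location enum.
; Shortly after BeginPlay it gets the cabbie from BP_RideManager and binds to its ride-ended event.
; Each tick it checks whether the cabbie overlaps it, stationary and holding a customer, then ends the ride and hides itself.
; Its construction script applies a dynamic pickup material with configurable colours and height-map texture.
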(event `self.ReceiveBeginPlay`
  (`self.SetActorHiddenInGame` true)
  (`KismetSystemLibrary.Delay` 0.1)
  (bind _returnvalue (`GameplayStatics.GetActorOfClass` "/Game/I01_Core/Blueprints/GameLogic/BP_RideManager.BP_RideManager_C"))
  (bind _output_get (set `self.RideManager` _returnvalue))
  (bind _output_get_2 (set `self.As BP Cabbie` (`/Game/I01_Core/Blueprints/GameLogic/BP_RideManager.BP_Cabbie` _output_get)))
  (add `/Game/I01_Core/Blueprints/Car/BP_Cabbie.OnRideEnded` _output_get_2 (`|CreateDelegate` :!event `EndRide`)))

(event `self.ReceiveTick`
  (params (DeltaSeconds :type "Float (single-precision)"))
  (bind _as_bp_cabbie (`self.As BP Cabbie`))
  (`self.RideManager`
    (:`then`
      (if (`KismetSystemLibrary.IsValid` _as_bp_cabbie)
        (if (and (`self.IsOverlappingActor` _as_bp_cabbie) (`/Game/I01_Core/Blueprints/Car/BP_Cabbie.HoldingCustomer` _as_bp_cabbie) (not (`/Game/I01_Core/Blueprints/Car/BP_Cabbie.IsCarMoving` _as_bp_cabbie)))
          ;[1 0.2604 0.2604] Will be replaces with picking up anim and UI anim calls
          (set `self.HasStopped` true)
          (`/Game/I01_Core/Blueprints/Car/BP_Cabbie.RideEnded` (`self.As BP Cabbie`))
          (`self.SetActorHiddenInGame` true)
          (set `self.HasStopped` false))))
    (:`else`)))

(event `EndRide`
  (`self.SetActorHiddenInGame` true))

(fn `UserConstructionScript`
  (bind _returnvalue (`PrimitiveComponent.CreateDynamicMaterialInstance` (`self.StaticMesh`) 0 "/Game/I01_Core/Assets/Materials/MI_CustomerPickup.MI_CustomerPickup" "None"))
  (bind _output_get (set `self.MaterialInstance` _returnvalue))
  (`MaterialInstanceDynamic.SetVectorParameterValue` _output_get "Colour" (`self.MaterialColour`))
  (`MaterialInstanceDynamic.SetTextureParameterValue` _output_get "Texture" "/Engine/Functions/Engine_MaterialFunctions02/ExampleContent/Textures/SineWaveHeightMap.SineWaveHeightMap")
  (`MaterialInstanceDynamic.SetVectorParameterValue` _output_get "GridColor" (`self.SecondaryColour`))
  (`TextRenderComponent.K2_SetText` (`self.TextRender`) (`KismetTextLibrary.Conv_StringToText` (`|GetEnumeratorNameAsString` (`self.Location`)))))