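; BP_Cabbie is the Maniac Cab car, which runs timed customer rides.
; BeginPlay caches the game state, assigns wheel and chassis meshes, and disables car input.
; SetupRide stores the customer, shows ride UI and derives a countdown from customer and game time, which Tick decrements until RideEnded.
; RideEnded passes bonus time and fare to GS_ManiacCab; delegate-style calls broadcast ride progress, while brake-light logic is disconnected.
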(event `self.ReceiveBeginPlay`
  (bind _asgs_maniac_cab (cast `/Game/I01_Core/Blueprints/GameLogic/GS_ManiacCab` (`GameplayStatics.GetGameState`))
    (:`then`
      (set `self.As GS Maniac Cab` _asgs_maniac_cab))
    (:`CastFailed`
      _))
  (set `self.BackLeftWheel` (`self.BackLeftWheelMeshParent`))
  (set `self.BackRightWheel` (`self.BackRightWheelMeshParent`))
  (set `self.FrontLeftWheel` (`self.FrontLeftWheelMeshParent`))
  (set `self.FrontRightWheel` (`self.FrontRightWheelMeshParent`))
  (set `self.CarChassis` (`self.Chassis`))
  (`self.EnableCarInput` false))

(event `self.ReceiveTick`
  (params (DeltaSeconds :type "Float (single-precision)"))
  (bind _milliseconds (`self.Milliseconds`))
  (if (== (`self.Seconds`) 0.0)
    (`/Engine/EditorBlueprintResources/StandardMacros.DoOnce` true :!label _label
      (:`Completed`
        (`self.RideEnded`)))
    (elif (`self.HoldingCustomer`)
      (`self.OnTimerUpdate`)
      (set `self.Milliseconds` (- _milliseconds DeltaSeconds))
      (if (<= _milliseconds -1.0)
        (set `self.Milliseconds` 0.0)
        (`/Engine/EditorBlueprintResources/StandardMacros.DecrementFloat` (`self.Seconds`)
          (:`  `
            (goto _label :!via `Reset`)))))))

(event `SetupRide`
  (params (CustomerData :type "/Game/I01_Core/Data/S_CustomerData Structure"))
  (bind _returnvalue (`KismetStringLibrary.Conv_StringToInt` (`/Game/I01_Core/Blueprints/GameLogic/GS_ManiacCab.CurrentTime` (`self.As GS Maniac Cab`))))
  (bind _output_get (set `self.CurrentCustomer` CustomerData))
  (`SceneComponent.SetVisibility` (`self.RideUI`) true false)
  (set `self.HoldingCustomer` true)
  (`/Game/I01_Core/Blueprints/GameLogic/GS_ManiacCab.AddRideTime` (`self.As GS Maniac Cab`))
  (bind ((`Time_11_9367EE94487BC509A653AF972D11280F` _time)) (break `/Game/I01_Core/Data/S_CustomerData` _output_get))
  (set `self.Seconds` (select `bool` (>= _time _returnvalue) :`false` (`KismetMathLibrary.Conv_IntToDouble` _time) :`true` (+ (`KismetMathLibrary.Conv_IntToDouble` _returnvalue) 20.0)))
  (`self.OnRideStarted` (`self.CurrentCustomer`)))

(event `RideEnded`
  (bind (_currentcustomer_time _currentcustomer_fare) (break `/Game/I01_Core/Data/S_CustomerData` (`self.CurrentCustomer`)))
  (`SceneComponent.SetVisibility` (`self.RideUI`) false true)
  (set `self.HoldingCustomer` false)
  (set `self.Milliseconds` 0.0)
  (`/Game/I01_Core/Blueprints/GameLogic/GS_ManiacCab.AddBonusTime` (`self.As GS Maniac Cab`) (`self.Seconds`) false)
  (`/Game/I01_Core/Blueprints/GameLogic/GS_ManiacCab.Update Player Score` (`self.As GS Maniac Cab`) _currentcustomer_fare)
  (`self.OnRideEnded`))

(fn `BrakeLights`
  (params (BrakeLights :type Boolean)))

(fn `IsCarMoving`
  (returns (ReturnValue :type Boolean))
  (return (> (`KismetMathLibrary.VSize` (`self.GetVelocity` self)) 8.0)))

(fn `UserConstructionScript`)