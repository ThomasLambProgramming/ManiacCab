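; Game timer component for Maniac Cab that runs a start countdown, then a match clock counting up or down, and ends the game through GM_ManiacCab.
; Tick either waits out the countdown delay or advances the clock by accumulating delta time into seconds.
; RepNotifies push formatted time and countdown state to GS_ManiacCab, which broadcasts updates.
; Bonus functions add seconds, with TriggerBonus also briefly pausing the clock.
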(event `self.ReceiveBeginPlay`
  (bind _asgs_maniac_cab (cast `/Game/I01_Core/Blueprints/GameLogic/GS_ManiacCab` (`GameplayStatics.GetGameState`)))
  (set `self.As GS Maniac Cab` _asgs_maniac_cab))

(event `self.ReceiveTick`
  (params (DeltaSeconds :type "Float (single-precision)"))
  (if (`self.CountdownRunning`)
    (`KismetSystemLibrary.Delay` (`self.Delay`))
    (set `self.CountdownRunning` false)
    (`/Game/I01_Core/Blueprints/GameLogic/GS_ManiacCab.CountdownEnded` (`self.As GS Maniac Cab`))
    (else
      (`self.RunGameTimer` DeltaSeconds (`self.MaxTime`)))))

(event `ToggleTimer`
  (params (EnableTimer :type Boolean) (EnableCountdown :type Boolean) (MaximumTime :type "Float (double-precision)"))
  (set `self.RunTimer` EnableTimer)
  (set `self.CountdownRunning` EnableCountdown)
  (if (`self.RunTimer`)
    (`/Engine/EditorBlueprintResources/StandardMacros.DoOnce` false :!label _label
      (:`Completed`
        (`self.SetMaximumTime` MaximumTime)))
    (else
      (goto _label :!via `Reset`))))

(event `TriggerBonus`
  (params (Time :type "Float (double-precision)") (PauseTime :type "Float (double-precision)"))
  (`self.AddBonusTime` Time)
  (`KismetSystemLibrary.Delay` 0.1)
  (set `self.RunTimer` false)
  (`KismetSystemLibrary.Delay` PauseTime)
  (set `self.RunTimer` true))

(fn `AddBonusTime`
  (params (Time :type "Float (double-precision)"))
  (set `self.Seconds` (+ (`self.Seconds`) Time)))

(fn `AddExtraRideTime`
  (set `self.Seconds` (+ (`self.Seconds`) 20.0)))

(fn `FormatTimer`
  (params (CurrentSeconds :type "Float (double-precision)") (CurrentMinutes :type "Float (double-precision)"))
  (returns (Time :type String))
  (if (`self.IsTimeIncreasing`)
    (return (`KismetTextLibrary.Conv_TextToString` (`|FormatText` "{m}.{s}" CurrentMinutes CurrentSeconds)))
    (else
      (return (`KismetStringLibrary.Conv_IntToString` (`KismetMathLibrary.Round` (`local.CurrentSeconds`)))))))

(fn `HasTimerEnded`
  (returns (ReturnValue :type Boolean))
  (bind (_returnvalue_days _returnvalue_hours _returnvalue_minutes _returnvalue_seconds) (`KismetMathLibrary.BreakTimespan` (`KismetMathLibrary.MakeTimespan` 0 0 0 (`KismetMathLibrary.FTrunc` (`self.MaxTime`)))))
  (return (select `bool` (`self.IsTimeIncreasing`) :`false` (and (== (`self.Minutes`) 0.0) (== (`self.Seconds`) 0.0)) :`true` (and (== (`self.Minutes`) _returnvalue_minutes) (== (`self.Seconds`) _returnvalue_seconds)))))

(fn `OnRep_CountdownRunning`
  (bind _as_gs_maniac_cab (`self.As GS Maniac Cab`))
  (bind _output_get (set `/Game/I01_Core/Blueprints/GameLogic/GS_ManiacCab.IsCountdownRunning` (`self.CountdownRunning`) _as_gs_maniac_cab))
  (`/Game/I01_Core/Blueprints/GameLogic/GS_ManiacCab.OnCountdownStarted` _as_gs_maniac_cab _output_get))

(fn `OnRep_CurrentTime`
  (bind _as_gs_maniac_cab (`self.As GS Maniac Cab`))
  (bind _output_get (set `/Game/I01_Core/Blueprints/GameLogic/GS_ManiacCab.CurrentTime` (`self.CurrentTime`) _as_gs_maniac_cab))
  (`/Game/I01_Core/Blueprints/GameLogic/GS_ManiacCab.OnTimeElapsedUpdated` _as_gs_maniac_cab _output_get))

(fn `OnRep_RunTimer`)

(fn `RunGameTimer`
  (params (`Delta Time` :type "Float (double-precision)") (MaxTime :type "Float (double-precision)"))
  (bind _milliseconds (`self.Milliseconds`))
  (bind _milliseconds_2 (`self.Milliseconds`))
  (bind _seconds (`self.Seconds`))
  (if (`self.RunTimer`)
    (bind _time (`self.FormatTimer` (`self.Seconds`) (`self.Minutes`)))
    (set `self.CurrentTime` _time)
    (if (not (`self.HasTimerEnded`))
      (if (`self.IsTimeIncreasing`)
        ;[0.2622 1 0.2033] Logic if time increases (0 -> 60)
        (if (`self.HasTimerEnded`)
          (set `self.RunTimer` false)
          (else
            (set `self.Milliseconds` (+ (`local.Delta Time`) _milliseconds_2))
            (if (>= _milliseconds_2 1.0)
              (set `self.Milliseconds` 0.0)
              (`/Engine/EditorBlueprintResources/StandardMacros.IncrementFloat` _seconds
                (:`  `
                  (if (>= _seconds 60.0)
                    (set `self.Seconds` 0.0)
                    (`/Engine/EditorBlueprintResources/StandardMacros.IncrementFloat` (`self.Minutes`))))))))
        (else
          ;[1 0.103 0.0831] Logic if time decreases (60 -> 0)
          (if (`self.HasTimerEnded`)
            (set `self.RunTimer` false)
            (else
              (set `self.Milliseconds` (- _milliseconds (`local.Delta Time`)))
              (if (<= _milliseconds -1.0)
                (set `self.Milliseconds` 0.0)
                (`/Engine/EditorBlueprintResources/StandardMacros.DecrementFloat` (`self.Seconds`)))))))
      (else
        (bind _asgm_maniac_cab (cast `/Game/I01_Core/Blueprints/GameLogic/GM_ManiacCab` (`GameplayStatics.GetGameMode`)))
        (`/Game/I01_Core/Blueprints/GameLogic/GM_ManiacCab.OnGameEnd` _asgm_maniac_cab)))))

(fn `SetMaximumTime`
  (params (MaximumTime :type "Float (double-precision)"))
  (if (`self.IsTimeIncreasing`)
    (set `self.MaxTime` (`local.MaximumTime`))
    (else
      (bind _output_get (set `self.Seconds` (`local.MaximumTime`)))))
  (bind _time (`self.FormatTimer` (select `bool` (`self.IsTimeIncreasing`) :`false` _output_get)))
  (set `self.CurrentTime` _time))