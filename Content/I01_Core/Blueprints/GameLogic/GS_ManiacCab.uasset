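; GS_ManiacCab is the game state for the Maniac Cab taxi game, tracking game start, ride count and total money earned.
; When the countdown ends, it sets HasGameStarted and enables car input on every cabbie pawn.
; Bonus time is tiered from the passed time value, broadcast, then sent to the timer component on GM_ManiacCab, cached under authority.
; The FreezePlayer branch and HasGameStarted RepNotify are empty.
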(event `self.ReceiveBeginPlay`
  (`/Engine/EditorBlueprintResources/ActorMacros.Switch Has Authority`
    (:`Authority`
      (bind _asgm_maniac_cab (cast `/Game/I01_Core/Blueprints/GameLogic/GM_ManiacCab` (`GameplayStatics.GetGameMode`)))
      (set `self.As GM Maniac Cab` _asgm_maniac_cab))))

(event `CountdownEnded`
  (set `self.HasGameStarted` true)
  (`self.ToggleAllPlayersMovement` true))

(event `ToggleAllPlayersMovement`
  (params (AllowInput :type Boolean))
  (for _array_element (`self.PlayerArray`)
    (bind _asps_cabbie (cast `/Game/I01_Core/Blueprints/Car/PS_Cabbie` _array_element))
    (bind _asbp_cabbie (cast `/Game/I01_Core/Blueprints/Car/BP_Cabbie` (`PlayerState.GetPawn` _asps_cabbie)))
    (`CarController.EnableCarInput` _asbp_cabbie AllowInput)))

(event `AddBonusTime`
  (params (Time :type "Float (double-precision)") (FreezePlayer :type Boolean))
  (bind _returnvalue (select `int` (`self.CheckRideSpeed` (`KismetMathLibrary.FTrunc` Time)) :`0` 0.0 :`1` 0.0 :`2` 2.0 :`3` 5.0))
  (if (!= _returnvalue 0.0)
    (`self.OnBonusTime` _returnvalue)
    (`/Game/I01_Core/Blueprints/GameLogic/BPC_GameTimer.TriggerBonus` (`/Game/I01_Core/Blueprints/GameLogic/GM_ManiacCab.BPC_GameTimer` (`self.As GM Maniac Cab`)) _returnvalue 3.0)
    (if FreezePlayer
      _)))

(event `AddRideTime`
  (`/Game/I01_Core/Blueprints/GameLogic/BPC_GameTimer.AddExtraRideTime` (`/Game/I01_Core/Blueprints/GameLogic/GM_ManiacCab.BPC_GameTimer` (`self.As GM Maniac Cab`))))

(fn `CheckRideSpeed`
  (params (Time :type Integer))
  (returns (SpeedIndex :type Integer))
  (if (> Time 8)
    (return 3)
    (elif (> Time 4)
      (return 2)
      (elif (<= Time 4)
        (return 1)
        (else
          (return 0))))))

(fn `OnRep_HasGameStarted`)

(fn `Update Player Score`
  (params (LastFare :type "Float (double-precision)"))
  (`/Engine/EditorBlueprintResources/StandardMacros.IncrementInt` (`self.RideCounter`)
    (:`  `
      (set `self.TotalMoney` (+ (`self.TotalMoney`) LastFare)))))

(fn `UserConstructionScript`)