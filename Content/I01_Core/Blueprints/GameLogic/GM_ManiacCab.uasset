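; Game mode for Maniac Cab that runs the timed match and starts the ride spawning.
; On BeginPlay it syncs the game timer component with the game state's time limit and delay, then spawns and attaches a ride manager.
; After a one-second delay, game start enables the countdown and tells the manager to spawn rides.
; A game end event stops the timer and flags the game state as finished.
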(event `self.ReceiveBeginPlay`
  (bind _asgs_maniac_cab (cast `/Game/I01_Core/Blueprints/GameLogic/GS_ManiacCab` (`GameplayStatics.GetGameState`)))
  (set `self.As GS Maniac Cab` _asgs_maniac_cab)
  (`/Game/I01_Core/Blueprints/GameLogic/BPC_GameTimer.SetMaximumTime` (`self.BPC_GameTimer`) (`/Game/I01_Core/Blueprints/GameLogic/GS_ManiacCab.TimeLimit` _asgs_maniac_cab))
  (set `/Game/I01_Core/Blueprints/GameLogic/GS_ManiacCab.Delay` (`/Game/I01_Core/Blueprints/GameLogic/BPC_GameTimer.Delay` (`self.BPC_GameTimer`)) _asgs_maniac_cab)
  (`self.CreateRideManager`)
  (`KismetSystemLibrary.Delay` 1.0)
  (`self.OnGameStart`))

(event `OnGameStart`
  (bind _as_gs_maniac_cab (`self.As GS Maniac Cab`)
    (:`then`
      (`/Game/I01_Core/Blueprints/GameLogic/BPC_GameTimer.ToggleTimer` (`self.BPC_GameTimer`) true true (`/Game/I01_Core/Blueprints/GameLogic/GS_ManiacCab.TimeLimit` _as_gs_maniac_cab))
      (`/Game/I01_Core/Blueprints/GameLogic/BP_RideManager.SpawnNewRides` (`self.RideManager`)))
    (:`else`)))

(event `OnGameEnd`
  (`/Game/I01_Core/Blueprints/GameLogic/BPC_GameTimer.ToggleTimer` (`self.BPC_GameTimer`) false false 0.0)
  (set `/Game/I01_Core/Blueprints/GameLogic/GS_ManiacCab.IsGameFinished` true (`self.As GS Maniac Cab`)))

(fn `CreateRideManager`
  (bind _returnvalue (`|SpawnActorFromClass` "/Game/I01_Core/Blueprints/GameLogic/BP_RideManager.BP_RideManager_C" (`KismetMathLibrary.MakeTransform` (0.0 0.0 0.0)) "Undefined" "MultiplyWithRoot" null null))
  (bind _output_get (set `self.RideManager` _returnvalue))
  (`self.K2_AttachToActor` _output_get self "None" "KeepRelative" "KeepRelative" "KeepRelative" true))

(fn `UserConstructionScript`)