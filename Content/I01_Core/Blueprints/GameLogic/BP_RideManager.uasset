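; Ride manager for a taxi game that spawns customer pickups around the player's BP_Cabbie and handles drop-off destinations.
; It caches all BP_DropOff actors and refreshes their distances to the cab every tick.
; Those distances drive recursive random destination selection within a range and ride-type tiers.
; While a customer is aboard, a spawned arrow points to the destination, hovering downward over it on overlap, with material-driven movement toggled.
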(event `self.ReceiveBeginPlay`
  (bind _outactors (`GameplayStatics.GetAllActorsOfClass` "/Game/I01_Core/Blueprints/Car/BP_DropOff.BP_DropOff_C"))
  (set `self.DropOffSpots` _outactors)
  (bind _asbp_cabbie (cast `/Game/I01_Core/Blueprints/Car/BP_Cabbie` (`GameplayStatics.GetPlayerPawn` 0)))
  (bind _output_get (set `self.BP_Cabbie` _asbp_cabbie))
  (add `/Game/I01_Core/Blueprints/Car/BP_Cabbie.OnRideEnded` _output_get (`|CreateDelegate` :!event `SpawnNewRides`))
  (for _array_element (`self.DropOffSpots`)
    (`KismetArrayLibrary.Array_Add` (`self.Distances`) (`KismetMathLibrary.Round` (`self.GetDistanceTo` _array_element (`self.BP_Cabbie`))))))

(event `self.ReceiveTick`
  (params (DeltaSeconds :type "Float (single-precision)"))
  (bind (_returnvalue_roll _returnvalue_pitch _returnvalue_yaw) (`KismetMathLibrary.BreakRotator` (`SceneComponent.K2_GetComponentRotation` (`/Game/I01_Core/Blueprints/Car/BP_Cabbie.Chassis` (`self.BP_Cabbie`)))))
  (bind _actor (`self.FindDropOffSpot` (`.Destination_10_83B772F44D83DE5A6036018E20FF6318` (break `/Game/I01_Core/Data/S_CustomerData` (`/Game/I01_Core/Blueprints/Car/BP_Cabbie.CurrentCustomer` (`self.BP_Cabbie`))))))
  (bind _returnvalue (`SceneComponent.K2_GetComponentLocation` (`/Game/I01_Core/Blueprints/Car/BP_DropOff.DefaultSceneRoot` _actor)))
  (bind (_x _y _z) (`KismetMathLibrary.BreakVector3f` _returnvalue))
  (set `self.Delta Seconds` DeltaSeconds)
  (`self.BP_Cabbie`
    (:`then`
      (`|ExecutionSequence`
        (:`then_0`
          (for (_array_element _array_index) (`self.DropOffSpots`)
            (`KismetArrayLibrary.Array_Set` (`self.Distances`) _array_index (`KismetMathLibrary.Round` (`self.GetDistanceTo` _array_element (`self.BP_Cabbie`))))))
        (:`then_1`
          (if (`/Game/I01_Core/Blueprints/Car/BP_Cabbie.HoldingCustomer` (`self.BP_Cabbie`))
            (`/Engine/EditorBlueprintResources/StandardMacros.IsValid` _actor
              (:`Is Valid`
                (`|ExecutionSequence`
                  (:`then_0`
                    (`/Engine/EditorBlueprintResources/StandardMacros.DoOnce` false :!label _label
                      (:`Completed`
                        (`self.SpawnArrow`))))
                  (:`then_1`
                    (`self.Arrow`
                      (:`then`
                        (if (not (`self.IsOverlappingActor` _actor (`self.BP_Cabbie`)))
                          (`SceneComponent.K2_SetWorldLocationAndRotation` (`Actor.RootComponent` (`self.Arrow`)) (`SceneComponent.K2_GetComponentLocation` (`/Game/I01_Core/Blueprints/Car/BP_Cabbie.Chassis` (`self.BP_Cabbie`))) (`KismetMathLibrary.FindLookAtRotation` (`SceneComponent.K2_GetComponentLocation` (`Actor.RootComponent` (`self.Arrow`))) _returnvalue) false false)
                          (`SceneComponent.K2_AddLocalOffset` (`Actor.RootComponent` (`self.Arrow`)) (`self.ArrowOffset`) false false)
                          (`|ExecutionSequence`
                            (:`then_0`
                              (`/Engine/EditorBlueprintResources/StandardMacros.DoOnce` false :!label _label_2
                                (:`Completed`
                                  (`self.ToggleArrowMovement` false))))
                            (:`then_1`
                              (goto _label_3 :!via `Reset`)))
                          (else
                            (`SceneComponent.K2_SetWorldLocationAndRotation` (`Actor.RootComponent` (`self.Arrow`)) (`KismetMathLibrary.VInterpTo` (`SceneComponent.K2_GetComponentLocation` (`Actor.RootComponent` (`self.Arrow`))) (`KismetMathLibrary.MakeVector` _x _y (+ _z 600.0)) (`self.Delta Seconds`) 4.0) (`KismetMathLibrary.MakeRotator` 0.0 -90.0 _returnvalue_yaw) false false)
                            (`|ExecutionSequence`
                              (:`then_0`
                                (`/Engine/EditorBlueprintResources/StandardMacros.DoOnce` false :!label _label_3
                                  (:`Completed`
                                    (`self.ToggleArrowMovement` true))))
                              (:`then_1`
                                (goto _label_2 :!via `Reset`))))))
                      (:`else`))))))
            (else
              (bind _arrow (`self.Arrow`)
                (:`then`
                  (`self.K2_DestroyActor` _arrow)
                  (goto _label :!via `Reset`))
                (:`else`)))))))
    (:`else`)))

(event `SpawnNewRides`
  (bind _bp_cabbie (`self.BP_Cabbie`))
  (bind _returnvalue (`self.K2_GetActorLocation` _bp_cabbie))
  (bind (_x _y) (`KismetMathLibrary.BreakVector3f` (+ (+ _returnvalue (* (`self.GetActorForwardVector` _bp_cabbie) 500.0)) (* (`KismetMathLibrary.RandomUnitVector`) (10000.0 10000.0 10000.0)))))
  (`/Engine/EditorBlueprintResources/StandardMacros.IsValid` _bp_cabbie
    (:`Is Valid`
      (for _ (range 7)
        (`|SpawnActorFromClass` "/Game/I01_Core/Blueprints/Car/BP_CustomerPickUp.BP_CustomerPickUp_C" (`KismetMathLibrary.MakeTransform` (`KismetMathLibrary.MakeVector` _x _y (+ (`.Z` (`KismetMathLibrary.BreakVector3f` _returnvalue)) 5.0))) "DontSpawnIfColliding" "MultiplyWithRoot" null null)))))

(event `ToggleArrowMovement`
  (params (MoveArrow :type Boolean))
  (`MaterialInstanceDynamic.SetScalarParameterValue` (`self.ArrowMaterial`) "Movement" (`KismetMathLibrary.Conv_BoolToDouble` MoveArrow)))

(fn `AssignLocation`
  (returns (Location :type "/Game/I01_Core/Data/E_Locations Enum"))
  (bind _location (`/Game/I01_Core/Blueprints/Car/BP_DropOff.Location` (`KismetArrayLibrary.Array_Random` (`self.DropOffSpots`))))
  (bind _returnvalue (/ (`self.FindDistance` _location) 100))
  (if (or (< _returnvalue 100) (> _returnvalue 2000))
    _
    (elif (`|EnumInequality` _location (`.Destination_10_83B772F44D83DE5A6036018E20FF6318` (break `/Game/I01_Core/Data/S_CustomerData` (`/Game/I01_Core/Blueprints/Car/BP_Cabbie.CurrentCustomer` (`self.BP_Cabbie`)))))
      (return _location)
      (else
        _)))
  (`self.AssignLocation`))

(fn `EvaluateRideType`
  (params (Distance :type Integer))
  (returns (TypeIndex :type Integer))
  (bind _distance (`local.Distance`))
  (if (> Distance 0)
    (if (<= _distance 30000)
      (return 0)
      (elif (<= _distance 60000)
        (return 1)
        (elif (<= _distance 100000)
          (return 2)
          (elif (> _distance 100000)
            (return 3)))))
    (else
      (`KismetSystemLibrary.PrintString` "Ride Type failed")
      (return 0))))

(fn `FindDistance`
  (params (Destination :type "/Game/I01_Core/Data/E_Locations Enum" :default "NewEnumerator0"))
  (returns (FoundDistance :type Integer))
  (locals (Distance :type Integer))
  (for (_array_element _array_index) (`self.DropOffSpots`)
    (if (`|EnumEquality` (`/Game/I01_Core/Blueprints/Car/BP_DropOff.Location` _array_element) Destination)
      (set `local.Distance` (`|GetArrayItem` (`self.Distances`) _array_index))
      (break)))
  (return (`local.Distance`)))

(fn `FindDropOffSpot`
  (params (Location :type "/Game/I01_Core/Data/E_Locations Enum" :default "NewEnumerator0"))
  (returns (Actor :type "/Game/I01_Core/Blueprints/Car/BP_DropOff Object Reference"))
  (locals (DropOff :type "/Game/I01_Core/Blueprints/Car/BP_DropOff Object Reference"))
  (for _array_element (`self.DropOffSpots`)
    (if (`|EnumEquality` (`/Game/I01_Core/Blueprints/Car/BP_DropOff.Location` _array_element) Location)
      (set `local.DropOff` _array_element)
      (break)))
  (return (`local.DropOff`)))

(fn `SpawnArrow`
  (bind _returnvalue (`|SpawnActorFromClass` "/Script/Engine.StaticMeshActor" (`KismetMathLibrary.MakeTransform` (+ (`SceneComponent.K2_GetComponentLocation` (`/Game/I01_Core/Blueprints/Car/BP_Cabbie.Chassis` (`self.BP_Cabbie`))) (`self.ArrowOffset`)) (struct) (0.7 0.7 0.7)) "Undefined" "MultiplyWithRoot" null null))
  (bind _output_get (set `self.Arrow` _returnvalue))
  (`StaticMeshActor.SetMobility` _output_get "Movable")
  (bind _staticmeshcomponent (`StaticMeshActor.StaticMeshComponent` _output_get))
  (`StaticMeshComponent.SetStaticMesh` _staticmeshcomponent "/Game/I01_Core/Assets/Models/SM_DirectionalArrow.SM_DirectionalArrow")
  (bind _returnvalue_2 (`PrimitiveComponent.CreateDynamicMaterialInstance` _staticmeshcomponent 0 "/Game/I01_Core/Assets/Materials/MI_DirectionalArrow.MI_DirectionalArrow" "None"))
  (set `self.ArrowMaterial` _returnvalue_2))

(fn `UserConstructionScript`)